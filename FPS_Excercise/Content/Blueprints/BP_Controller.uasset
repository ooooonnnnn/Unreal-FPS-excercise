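; Player controller that turns Enhanced Input actions into movement, look and shoot commands.
; It adds the MC_Game mapping context on BeginPlay.
; Move applies normalized input relative to the player character's transform, and look feeds yaw and pitch to the controller, both looked up by player index 0.
; Shoot is forwarded through the BP_IShootInputConsumer interface, cached from the pawn on possession, decoupling input from the pawn's shooting logic.
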(event `self.ReceiveBeginPlay`
  (`EnhancedInputSubsystemInterface.AddMappingContext` (subsystem `EnhancedInputLocalPlayerSubsystem`) "/Game/Blueprints/Input/MC_Game.MC_Game" 0 (struct)))

(event `EnhancedInput|/Game/Blueprints/Input/IA_Move`
  (params (ActionValue :type "Vector2D Structure") (ElapsedSeconds :type "Float (double-precision)") (TriggeredSeconds :type "Float (double-precision)") (InputAction :type "InputAction Object Reference" :default "/Game/Blueprints/Input/IA_Move.IA_Move"))
  (bind _returnvalue (`GameplayStatics.GetPlayerCharacter` 0))
  (:`Triggered`
    (`Pawn.AddMovementInput` _returnvalue (`KismetMathLibrary.TransformDirection` (`self.GetTransform` _returnvalue) (`KismetMathLibrary.Conv_Vector2DToVector` (`KismetMathLibrary.Normal2D` ActionValue))) 1.0 false)))

(event `EnhancedInput|/Game/Blueprints/Input/IA_Look`
  (params (ActionValue :type "Vector2D Structure") (ElapsedSeconds :type "Float (double-precision)") (TriggeredSeconds :type "Float (double-precision)") (InputAction :type "InputAction Object Reference" :default "/Game/Blueprints/Input/IA_Look.IA_Look"))
  (bind (_x _y) (`KismetMathLibrary.BreakVector2D` ActionValue))
  (bind _returnvalue (`GameplayStatics.GetPlayerController` 0))
  (:`Triggered`
    (`self.AddYawInput` _returnvalue _x)
    (`self.AddPitchInput` _returnvalue _y)))

(event `EnhancedInput|/Game/Blueprints/Input/IA_Shoot`
  (params (ActionValue :type Boolean) (ElapsedSeconds :type "Float (double-precision)") (TriggeredSeconds :type "Float (double-precision)") (InputAction :type "InputAction Object Reference" :default "/Game/Blueprints/Input/IA_Shoot.IA_Shoot"))
  (:`Triggered`
    (`/Game/Blueprints/Interfaces/BP_IShootInputConsumer.Shoot` (stale `self.ReceivePossess` _asbp_ishoot_input_consumer))))

(event `self.ReceivePossess`
  (params (PossessedPawn :type "Pawn Object Reference"))
  (bind _asbp_ishoot_input_consumer (cast `/Game/Blueprints/Interfaces/BP_IShootInputConsumer` PossessedPawn)))

(fn `UserConstructionScript`)