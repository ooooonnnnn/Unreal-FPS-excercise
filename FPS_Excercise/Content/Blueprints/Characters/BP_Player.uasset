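; BP_Player is the player character Blueprint, handling gun use, item switching and health.
; Its Inventory's item-changed event updates the current gun when the new item is a BP_Gun_Base, and shoot input fires that gun if valid.
; Next-item input scrolls the Inventory.
; Damage subtracts from current health, which regenerates every Tick at a set rate, capped at the starting value, with no death handling.
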(event `self.ReceiveBeginPlay`
  (`|ExecutionSequence`
    (:`then_0`
      (add `/Game/Blueprints/BP_Inventory.On Item Changed` (`self.Inventory`) (delegate `Update current gun`)))
    (:`then_1`
      (set `self.Current Health` (`self.Starting Health`)))))

(event `Update current gun`
  (params (`Current Item` :type "/Game/Blueprints/Interfaces/BP_IEquippable Interface"))
  (bind _asbp_gun_base (cast `/Game/Blueprints/Items/Guns/BP_Gun_Base` `Current Item`))
  (set `self.Current Gun` _asbp_gun_base))

(event `/Game/Blueprints/Interfaces/BP_IFPSInputConsumer.Handle Shoot Input`
  (bind _current_gun (`self.Current Gun`))
  (`/Engine/EditorBlueprintResources/StandardMacros.IsValid` _current_gun
    (:`Is Valid`
      (`/Game/Blueprints/Items/Guns/BP_Gun_Base.Shoot` _current_gun))))

(event `/Game/Blueprints/Interfaces/BP_IFPSInputConsumer.Handle Next Item Input`
  (`/Game/Blueprints/BP_Inventory.Scroll To Next Item` (`self.Inventory`)))

(event `self.ReceiveTick`
  (params (DeltaSeconds :type "Float (single-precision)"))
  (`self.Regenerate Health` DeltaSeconds))

(event `/Game/Blueprints/Interfaces/BP_IDamagable.Take Damage`
  (params (`Damage Amount` :type "Float (double-precision)"))
  (set `self.Current Health` (- (`self.Current Health`) `Damage Amount`)))

(fn `Regenerate Health`
  (params (`Delta Seconds` :type "Float (double-precision)"))
  (set `self.Current Health` (`KismetMathLibrary.FMin` (+ (`self.Current Health`) (* `Delta Seconds` (`self.Health Regeneration Rate`))) (`self.Starting Health`))))

(fn `UserConstructionScript`)