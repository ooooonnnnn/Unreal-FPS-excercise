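; Enemy character that patrols, spots and chases the player, and loses the game for the player on contact.
; A tick-driven, timed state machine switches between Patrolling, Watching and Chasing using squared-distance and line-trace sight checks, broadcasting each change; movement itself is not handled here.
; Chasing ends only on timeout, regardless of sight.
; It registers with the game mode on spawn and unregisters when damage destroys it.
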(event `self.ReceiveBeginPlay`
  (`|ExecutionSequence`
    (:`then_0`
      ;[1 1 1] Set starting health and vision distance
      (set `self.Current Health` (`self.Starting Health`))
      (set `self.Vision Square Distance` (`KismetMathLibrary.MultiplyMultiply_FloatFloat` (`self.Vision Distance`) 2.0)))
    (:`then_1`
      (set `self. Player Pawn` (`GameplayStatics.GetPlayerPawn` 0)))
    (:`then_2`
      ;[1 1 1] Sign up in the game mode
      (bind _asbp_my_game_mode (cast `/Game/Blueprints/BP_MyGameMode` (`GameplayStatics.GetGameMode`)))
      (bind _output_get (set `self.Game Mode` _asbp_my_game_mode))
      (`KismetArrayLibrary.Array_Add` (`/Game/Blueprints/BP_MyGameMode.Alive Enemies` _output_get) self))))

(event `/Game/Blueprints/Interfaces/BP_IDamagable.Take Damage`
  (params (`Damage Amount` :type "Float (double-precision)"))
  (`|ExecutionSequence`
    (:`then_0`
      (bind _output_get (set `self.Current Health` (- (`self.Current Health`) `Damage Amount`)))
      (if (<= _output_get 0.0)
        (`/Game/Blueprints/BP_MyGameMode.Remove Enemy` (`self.Game Mode`) self)
        (`self.K2_DestroyActor`)))
    (:`then_1`
      (`KismetSystemLibrary.PrintString` (`KismetStringLibrary.Concat_StrStr` (`KismetSystemLibrary.GetDisplayName` self) " has " (`KismetStringLibrary.Conv_DoubleToString` (`self.Current Health`)) " health left") true true (struct :`R` 0.088721 :`G` 1.0 :`A` 1.0) 5.0))))

(event `self.ReceiveTick`
  (params (DeltaSeconds :type "Float (single-precision)"))
  (bind _returnvalue (and (<= (`KismetMathLibrary.Vector_DistanceSquared` (`self.K2_GetActorLocation` (`self. Player Pawn`)) (`self.K2_GetActorLocation`)) (`self.Vision Square Distance`)) (`self.Can See Player`)))
  ;[1 1 1] State Machine
  (`|ExecutionSequence`
    (:`then_0`
      (set `self.Timer` (+ (`self.Timer`) DeltaSeconds)))
    (:`then_1`
      (switch `/Game/Blueprints/Enums/EnemyState` (`self.Movement State`)
        (:`NewEnumerator0`
          (if _returnvalue
            (bind _output_get (set `self.Movement State` "NewEnumerator1"))
            (set `self.Timer` 0.0)
            (`self.On State Change` _output_get)))
        (:`NewEnumerator1`
          (if _returnvalue
            (if (>= (`self.Timer`) (`self.Watch Time`))
              (set `self.Timer` 0.0)
              (bind _output_get_2 (set `self.Movement State` "NewEnumerator2"))
              (`self.On State Change` _output_get_2))
            (else
              (set `self.Timer` 0.0)
              (bind _output_get_3 (set `self.Movement State` "NewEnumerator0"))
              (`self.On State Change` _output_get_3))))
        (:`NewEnumerator2`
          (if (>= (`self.Timer`) (`self.Chase Time`))
            (set `self.Timer` 0.0)
            (bind _output_get_4 (set `self.Movement State` "NewEnumerator0"))
            (`self.On State Change` _output_get_4)))))))

(event `self.ReceiveHit`
  (params (MyComp :type "PrimitiveComponent Object Reference") (Other :type "Actor Object Reference") (OtherComp :type "PrimitiveComponent Object Reference") (bSelfMoved :type Boolean) (HitLocation :type "Vector Structure") (HitNormal :type "Vector Structure") (NormalImpulse :type "Vector Structure") (Hit :type "HitResult Structure (by ref)"))
  (cast `/Game/Blueprints/Characters/BP_Player` Other)
  (bind _asbp_my_game_mode (cast `/Game/Blueprints/BP_MyGameMode` (`GameplayStatics.GetGameMode`)))
  (`/Game/Blueprints/BP_MyGameMode.Lose Game` _asbp_my_game_mode))

(fn `Can See Player`
  (returns (`Can See Player` :type Boolean))
  (bind (_outhit _returnvalue) (`KismetSystemLibrary.LineTraceSingleForObjects` :`Start` (`self.K2_GetActorLocation` self) :`End` (`self.K2_GetActorLocation` (`self. Player Pawn`)) :`ObjectTypes` (`|MakeArray` "ObjectTypeQuery1" "ObjectTypeQuery2" "ObjectTypeQuery3" :!type "EObjectTypeQuery Enum") :`DrawDebugType` "ForOneFrame"))
  (if _returnvalue
    (cast `/Game/Blueprints/Characters/BP_Player` (`.HitActor` (`GameplayStatics.BreakHitResult` _outhit))
      (:`then`
        (return true))
      (:`CastFailed`
        (return false)))))

(fn `UserConstructionScript`)