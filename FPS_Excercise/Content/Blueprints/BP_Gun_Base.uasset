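; BP_Gun_Base is a gun Blueprint that fires a single shot on BeginPlay.
; Shoot checks and decrements CurrentBullets, then spawns a Bullet actor at the BulletExit transform.
; It launches the bullet by setting linear velocity on its physics Model along BulletExit's forward vector, scaled by BulletExitVelocity.
; The ammo check also passes at zero, and debug strings report shots and an empty gun.
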(event `self.ReceiveBeginPlay`
  (`self.Shoot`))

(fn `Shoot`
  (if (>= (`self.Current Bullets`) 0)
    (`/Engine/EditorBlueprintResources/StandardMacros.DecrementInt` (`self.Current Bullets`)
      (:`  `
        (`KismetSystemLibrary.PrintString` "Shoot")
        (bind _returnvalue (`|SpawnActorFromClass` "/Game/Blueprints/Bullet.Bullet_C" (`SceneComponent.K2_GetComponentToWorld` (`self.Bullet Exit`)) "AlwaysSpawn" "MultiplyWithRoot" null 0.0 null))
        (`PrimitiveComponent.SetPhysicsLinearVelocity` (`/Game/Blueprints/Bullet.Model` _returnvalue) (* (`SceneComponent.GetForwardVector` (`self.Bullet Exit`)) (`self.Bullet Exit Velocity`)) false "None")))
    (else
      (`KismetSystemLibrary.PrintString` "No more bullets"))))

(fn `UserConstructionScript`)