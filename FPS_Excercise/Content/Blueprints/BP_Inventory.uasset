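; BP_Inventory is an inventory Blueprint that switches which of its held items is equipped.
; EquipItem loops over the Items array, equips the entry at the requested index and unequips all others, printing each item's actor name as a debug message.
; CanPickItem is a stub that always returns false, and the event graph is empty apart from disabled default events.
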(fn `Can Pick Item`
  (params (`Item to Pick` :type "/Game/Blueprints/Interfaces/BP_IPickable Interface"))
  (returns (`Can Pick` :type Boolean))
  (return false))

(fn `Equip Item`
  (params (`Item Index to Equip` :type Integer))
  (locals (NewLocalVar :type Integer))
  (for (_array_element _array_index) (`self.Items`)
    (bind _actor (`/Game/Blueprints/Interfaces/BP_IEquippable.Get Actor` _array_element))
    (if (== _array_index `Item Index to Equip`)
      (bind _returnvalue (`KismetSystemLibrary.GetDisplayName` _actor))
      (`KismetSystemLibrary.PrintString` (`KismetStringLibrary.Concat_StrStr` "Equipping " _returnvalue))
      (`/Game/Blueprints/Interfaces/BP_IEquippable.Equip` _array_element true)
      (else
        (`KismetSystemLibrary.PrintString` (`KismetStringLibrary.Concat_StrStr` "Unequipping " _returnvalue))
        (`/Game/Blueprints/Interfaces/BP_IEquippable.Equip` _array_element false)))))