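; AI controller for BP_Enemy that patrols, watches or chases the player according to the enemy's movement state.
; State change events reset the patrol flag or stop movement, while Tick runs each behavior.
; Patrolling loops through the enemy's target actors, using a Busy flag to issue one move at a time.
; Watching steers yaw by the forward-to-player cross product's Z, without delta-time scaling; chasing reissues AIMoveTo every tick.
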(event `self.ReceiveBeginPlay`
  (`|ExecutionSequence`
    (:`then_0`
      (set `self.Player Pawn` (`GameplayStatics.GetPlayerPawn` 0)))
    (:`then_1`
      (set `self.Patrol Targets` (`/Game/Blueprints/Characters/BP_Enemy.Patrol Targets` (`self.Controlled Enemy`))))))

(event `self.ReceivePossess`
  (params (PossessedPawn :type "Pawn Object Reference"))
  (bind _asbp_enemy (cast `/Game/Blueprints/Characters/BP_Enemy` PossessedPawn))
  (bind _output_get (set `self.Controlled Enemy` _asbp_enemy))
  (add `/Game/Blueprints/Characters/BP_Enemy.On State Change` _output_get (delegate `On State Change`)))

(event `On State Change`
  (params (`New State` :type "/Game/Blueprints/Enums/EnemyState Enum" :default "NewEnumerator0"))
  (switch `/Game/Blueprints/Enums/EnemyState` `New State`
    (:`NewEnumerator0`
      (set `self.Busy` false))
    (:`NewEnumerator1`
      (`self.StopMovement`))))

(event `self.ReceiveTick`
  (params (DeltaSeconds :type "Float (single-precision)"))
  (bind (_returnvalue_x _returnvalue_y _returnvalue_z) (`KismetMathLibrary.BreakVector` (`KismetMathLibrary.Cross_VectorVector` (`KismetMathLibrary.Normal` (- (`self.K2_GetActorLocation` (`self.Player Pawn`)) (`self.K2_GetActorLocation` (`self.Controlled Enemy`)))) (`self.GetActorForwardVector` (`self.Controlled Enemy`)))))
  (switch `/Game/Blueprints/Enums/EnemyState` (`/Game/Blueprints/Characters/BP_Enemy.Movement State` (`self.Controlled Enemy`))
    (:`NewEnumerator0`
      (if (not (`self.Busy`))
        (set `self.Busy` true)
        (`|AIMoveTo` (`self.Controlled Enemy`) (0.0 0.0 0.0) (`|GetArrayItem` (`self.Patrol Targets`) (`self.Current Patrol Index`))
          (:`OnSuccess`
            (bind _result (`/Engine/EditorBlueprintResources/StandardMacros.IncrementInt` (`self.Current Patrol Index`))
              (:`  `
                (set `self.Current Patrol Index` (mod _result (`KismetArrayLibrary.Array_Length` (`self.Patrol Targets`))))
                (set `self.Busy` false)))))))
    (:`NewEnumerator1`
      (`self.K2_AddActorLocalRotation` (`self.Controlled Enemy`) (`KismetMathLibrary.MakeRotator` 0.0 0.0 (* (* _returnvalue_z -1.0) (`self.Look Rotation Rate`))) false false))
    (:`NewEnumerator2`
      (`|AIMoveTo` (`self.Controlled Enemy`) (0.0 0.0 0.0) (`self.Player Pawn`)))))

(fn `UserConstructionScript`)