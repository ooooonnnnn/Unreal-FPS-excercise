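; BP_Controller is an FPS player controller that maps Enhanced Input to movement, look, shooting and item switching.
; It adds the game mapping context on begin play, then applies move input relative to the player character and look input as yaw and pitch.
; Shoot and next-item presses fire dispatchers, bound on possess to forward to the pawn through BP_IFPSInputConsumer and cleared on unpossess.
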(event `self.ReceiveBeginPlay`
  (`EnhancedInputSubsystemInterface.AddMappingContext` (subsystem `EnhancedInputLocalPlayerSubsystem`) "/Game/Blueprints/Input/MC_Game.MC_Game" 0 (struct)))

(event `EnhancedInput|/Game/Blueprints/Input/IA_Move`
  (params (ActionValue :type "Vector2D Structure") (ElapsedSeconds :type "Float (double-precision)") (TriggeredSeconds :type "Float (double-precision)") (InputAction :type "InputAction Object Reference" :default "/Game/Blueprints/Input/IA_Move.IA_Move"))
  (bind _returnvalue (`GameplayStatics.GetPlayerCharacter` 0))
  (:`Triggered`
    (`Pawn.AddMovementInput` _returnvalue (`KismetMathLibrary.TransformDirection` (`self.GetTransform` _returnvalue) (`KismetMathLibrary.Conv_Vector2DToVector` (`KismetMathLibrary.Normal2D` ActionValue))) 1.0 false)))

(event `EnhancedInput|/Game/Blueprints/Input/IA_Look`
  (params (ActionValue :type "Vector2D Structure") (ElapsedSeconds :type "Float (double-precision)") (TriggeredSeconds :type "Float (double-precision)") (InputAction :type "InputAction Object Reference" :default "/Game/Blueprints/Input/IA_Look.IA_Look"))
  (bind (_x _y) (`KismetMathLibrary.BreakVector2D` ActionValue))
  (bind _returnvalue (`GameplayStatics.GetPlayerController` 0))
  (:`Triggered`
    (`self.AddYawInput` _returnvalue _x)
    (`self.AddPitchInput` _returnvalue _y)))

(event `EnhancedInput|/Game/Blueprints/Input/IA_Shoot`
  (params (ActionValue :type Boolean) (ElapsedSeconds :type "Float (double-precision)") (TriggeredSeconds :type "Float (double-precision)") (InputAction :type "InputAction Object Reference" :default "/Game/Blueprints/Input/IA_Shoot.IA_Shoot"))
  (:`Triggered`
    (`self.Shoot`)))

(event `EnhancedInput|/Game/Blueprints/Input/IA_NextItem`
  (params (ActionValue :type Boolean) (ElapsedSeconds :type "Float (double-precision)") (TriggeredSeconds :type "Float (double-precision)") (InputAction :type "InputAction Object Reference" :default "/Game/Blueprints/Input/IA_NextItem.IA_NextItem"))
  (:`Triggered`
    (`self.Next Item`)))

(event `self.ReceivePossess`
  (params (PossessedPawn :type "Pawn Object Reference"))
  (bind _asbp_ifpsinput_consumer (cast `/Game/Blueprints/Interfaces/BP_IFPSInputConsumer` PossessedPawn))
  ;[1 1 1] Subscribe character to fps input events
  (`|ExecutionSequence`
    (:`then_0`
      (add `self.Shoot` (delegate `Handle Shoot Input`)))
    (:`then_1`
      (add `self.Next Item` (delegate `Handle Next Item Input`)))))

(event `Handle Shoot Input`
  ;[1 1 1] Subscribe character to fps input events
  (`/Game/Blueprints/Interfaces/BP_IFPSInputConsumer.Handle Shoot Input` (stale `self.ReceivePossess` _asbp_ifpsinput_consumer)))

(event `Handle Next Item Input`
  ;[1 1 1] Subscribe character to fps input events
  (`/Game/Blueprints/Interfaces/BP_IFPSInputConsumer.Handle Next Item Input` (stale `self.ReceivePossess` _asbp_ifpsinput_consumer)))

(event `self.ReceiveUnPossess`
  (params (UnpossessedPawn :type "Pawn Object Reference"))
  (`|ExecutionSequence`
    (:`then_0`
      (clear `self.Shoot`))
    (:`then_1`
      (clear `self.Next Item`))))

(fn `UserConstructionScript`)