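; Base gun actor that can be picked up, equipped, fired and refilled with magazines.
; Shoot spends a round and launches a physics-driven BP_Bullet from BulletExit, passing damage and trail color, then reports success or an empty gun through OnShoot.
; Pickup attaches the gun to a socket with an offset, while Equip toggles visibility and firing.
; Magazines are accepted only if their type matches and all rounds fit, and adding one calls OnReload.
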(event `/Game/Blueprints/Interfaces/BP_IEquippable.Equip`
  (params (`Equip State` :type Boolean))
  (`|ExecutionSequence`
    (:`then_0`
      (set `self.Can Shoot` `Equip State`)
      (`self.SetActorHiddenInGame` (not `Equip State`)))))

(event `/Game/Blueprints/Interfaces/BP_IEquippable.Add Pickable`
  (params (Pickable :type "/Game/Blueprints/Interfaces/BP_IPickable Interface"))
  ;[1 1 1] Get bullets when picking up a magazine
  (bind _amount (`/Game/Blueprints/Interfaces/BP_IPickable.Amount` Pickable))
  (set `self.Current Bullets` (+ _amount (`self.Current Bullets`)))
  (`self.OnReload`))

(fn `Allow Other Pickable`
  (params (Pickable :type "/Game/Blueprints/Interfaces/BP_IPickable Interface"))
  (returns (`Can Pick` :type Boolean))
  (locals (_Pickable :type "/Game/Blueprints/Interfaces/BP_IPickable Interface"))
  (bind _output_get (set `local._Pickable` Pickable))
  (bind _item_type (`/Game/Blueprints/Interfaces/BP_IPickable.Get Item Type` _output_get))
  (if (`|EnumEquality` _item_type (`self.Bullet Type`))
    (bind _amount (`/Game/Blueprints/Interfaces/BP_IPickable.Amount` (`local._Pickable`)))
    (return (<= _amount (- (`self.Max Bullets`) (`self.Current Bullets`))))
    (else
      (return false))))

(fn `Amount`
  (returns (Amount :type Integer))
  (return (`self.Current Bullets`)))

(fn `Get Actor`
  (returns (Actor :type "Actor Object Reference"))
  (return self))

(fn `Get Item Type`
  (returns (`Item Type` :type "/Game/Blueprints/Enums/ItemType Enum"))
  (return "NewEnumerator0"))

(fn `Is Pickable`
  (returns (`Is Pickable` :type Boolean))
  (return (`self.Pickable`)))

(fn `Pick Up`
  (params (`New Parent` :type "Actor Object Reference") (`Socket Name` :type Name))
  (returns (`Amount Picked` :type Integer))
  (`|ExecutionSequence`
    (:`then_0`
      (set `self.Pickable` false))
    (:`then_1`
      (`self.K2_AttachToActor` `New Parent` `Socket Name` "SnapToTarget" "SnapToTarget" "KeepRelative")
      (`self.K2_AddActorLocalOffset` (`self.Delta Position From Eyes`)))
    (:`then_2`
      (return (`self.Current Bullets`)))))

(fn `Shoot`
  (if (`self.Can Shoot`)
    (if (> (`self.Current Bullets`) 0)
      (`|ExecutionSequence`
        (:`then_0`
          ;[1 1 1] Shooting the bullet
          (`/Engine/EditorBlueprintResources/StandardMacros.DecrementInt` (`self.Current Bullets`)
            (:`  `
              (bind _returnvalue (`|SpawnActorFromClass` "/Game/Blueprints/Items/BP_Bullet.BP_Bullet_C" (`SceneComponent.K2_GetComponentToWorld` (`self.Bullet Exit`)) "AlwaysSpawn" "MultiplyWithRoot" null (`self.Damage`) (`self.Bullet Trail Color`) null))
              (`PrimitiveComponent.SetPhysicsLinearVelocity` (`/Game/Blueprints/Items/BP_Bullet.Model` _returnvalue) (* (`SceneComponent.GetForwardVector` (`self.Bullet Exit`)) (`self.Bullet Exit Velocity`)) false "None"))))
        (:`then_1`
          (`self.OnShoot` true)))
      (else
        (`self.OnShoot` false)))))

(fn `UserConstructionScript`)