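; BP_Magazine_Base is a base Blueprint for magazine items that supply bullets when picked up.
; It is always pickable and reports NumberOfBullets as its amount and BulletType as its item type.
; Pick Up destroys the actor, prints a debug string and returns the bullet count, ignoring the parent and socket inputs.
; PartialPickUp is an empty event, so the base has no partial pickup behavior.
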(event `/Game/Blueprints/Interfaces/BP_IPickable.Partial Pick Up`
  (params (`Amount to Pick` :type Integer)))

(fn `Amount`
  (returns (Amount :type Integer))
  (return (`self.Number of Bullets`)))

(fn `Get Item Type`
  (returns (`Item Type` :type "/Game/Blueprints/Enums/ItemType Enum"))
  (return (`self.Bullet Type`)))

(fn `Is Pickable`
  (returns (`Is Pickable` :type Boolean))
  (return true))

(fn `Pick Up`
  (params (`New Parent` :type "Actor Object Reference") (`Socket Name` :type Name))
  (returns (`Amount Picked` :type Integer))
  (`|ExecutionSequence`
    (:`then_0`
      (`self.K2_DestroyActor`)
      (`KismetSystemLibrary.PrintString` "I got picked"))
    (:`then_1`
      (return (`self.Number of Bullets`)))))

(fn `UserConstructionScript`)