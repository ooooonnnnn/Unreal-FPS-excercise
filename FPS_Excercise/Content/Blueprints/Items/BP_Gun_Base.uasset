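; BP_Gun_Base is a base gun actor that can be picked up, equipped and fired.
; PickUp snaps it to a parent socket with an offset, while Equip toggles visibility and the ability to shoot.
; Shoot consumes a bullet, spawns a BP_Bullet at BulletExit with the gun's damage, launches it by physics velocity and calls the OnShoot dispatcher.
; Reload is an empty stub, and debug strings report equip state and empty ammo.
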(event `/Game/Blueprints/Interfaces/BP_IPickable.Pick Up`
  (params (`New Parent` :type "Actor Object Reference") (`Socket Name` :type Name))
  (`self.K2_AttachToActor` `New Parent` `Socket Name` "SnapToTarget" "SnapToTarget" "KeepRelative")
  (`self.K2_AddActorLocalOffset` (`self.Delta Position From Eyes`)))

(event `/Game/Blueprints/Interfaces/BP_IEquippable.Equip`
  (params (`Equip State` :type Boolean))
  (`|ExecutionSequence`
    (:`then_0`
      (set `self.Can Shoot` `Equip State`)
      (`self.SetActorHiddenInGame` (not `Equip State`)))
    (:`then_1`
      (`KismetSystemLibrary.PrintString` (`KismetStringLibrary.Concat_StrStr` (`KismetSystemLibrary.GetDisplayName` self) (`KismetMathLibrary.SelectString` " is equipped" " is unequipped" `Equip State`))))))

(fn `Get Actor`
  (returns (Actor :type "Actor Object Reference"))
  (return self))

(fn `Reload`)

(fn `Shoot`
  (if (`self.Can Shoot`)
    (if (> (`self.Current Bullets`) 0)
      (`|ExecutionSequence`
        (:`then_0`
          ;[1 1 1] Shooting the bullet
          (`/Engine/EditorBlueprintResources/StandardMacros.DecrementInt` (`self.Current Bullets`)
            (:`  `
              (bind _returnvalue (`|SpawnActorFromClass` "/Game/Blueprints/Items/BP_Bullet.BP_Bullet_C" (`SceneComponent.K2_GetComponentToWorld` (`self.Bullet Exit`)) "AlwaysSpawn" "MultiplyWithRoot" null (`self.Damage`) null))
              (`PrimitiveComponent.SetPhysicsLinearVelocity` (`/Game/Blueprints/Items/BP_Bullet.Model` _returnvalue) (* (`SceneComponent.GetForwardVector` (`self.Bullet Exit`)) (`self.Bullet Exit Velocity`)) false "None"))))
        (:`then_1`
          (`self.OnShoot`)))
      (else
        (`KismetSystemLibrary.PrintString` "No more bullets")))))

(fn `UserConstructionScript`)