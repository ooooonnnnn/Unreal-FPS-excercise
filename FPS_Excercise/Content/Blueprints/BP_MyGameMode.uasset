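; BP_MyGameMode is a game mode that decides when the player wins or loses.
; RemoveEnemy takes a given enemy out of the AliveEnemies list and triggers WinGame once the list is empty.
; WinGame and LoseGame only print a colored on-screen message, and nothing in this file fills the list or calls LoseGame.
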(fn `Lose Game`
  (`KismetSystemLibrary.PrintString` "You Lost!" true true (struct :`R` 1.0 :`G` 0.011604 :`A` 1.0) 30.0 "Lose Game"))

(fn `Remove Enemy`
  (params (`Enemy To Kill` :type "/Game/Blueprints/Characters/BP_Enemy Object Reference"))
  (`KismetArrayLibrary.Array_RemoveItem` (`self.Alive Enemies`) `Enemy To Kill`)
  (if (<= (`KismetArrayLibrary.Array_Length` (`self.Alive Enemies`)) 0)
    (`self.Win Game`)))

(fn `UserConstructionScript`)

(fn `Win Game`
  (`KismetSystemLibrary.PrintString` "You Win!" true true (struct :`G` 1.0 :`B` 0.019231 :`A` 1.0) 30.0 "Win Game"))