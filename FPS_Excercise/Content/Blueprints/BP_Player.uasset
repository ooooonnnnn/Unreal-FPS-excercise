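; BP_Player is the player Blueprint that fires the currently equipped gun and scrolls through inventory items.
; On BeginPlay it binds to the Inventory's item-changed event and caches the new item as CurrentGun when it casts to BP_Gun_Base.
; An item that fails the cast leaves the previous gun cached.
; The shoot input handler fires CurrentGun if valid, and the next-item handler scrolls the Inventory.
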(event `self.ReceiveBeginPlay`
  (add `/Game/Blueprints/BP_Inventory.On Item Changed` (`self.Inventory`) (delegate `Update current gun`)))

(event `Update current gun`
  (params (`Current Item` :type "/Game/Blueprints/Interfaces/BP_IEquippable Interface"))
  (bind _asbp_gun_base (cast `/Game/Blueprints/Items/Guns/BP_Gun_Base` `Current Item`))
  (set `self.Current Gun` _asbp_gun_base))

(event `/Game/Blueprints/Interfaces/BP_IFPSInputConsumer.Handle Shoot Input`
  (bind _current_gun (`self.Current Gun`))
  (`/Engine/EditorBlueprintResources/StandardMacros.IsValid` _current_gun
    (:`Is Valid`
      (`/Game/Blueprints/Items/Guns/BP_Gun_Base.Shoot` _current_gun))))

(event `/Game/Blueprints/Interfaces/BP_IFPSInputConsumer.Handle Next Item Input`
  (`/Game/Blueprints/BP_Inventory.Scroll To Next Item` (`self.Inventory`)))

(fn `UserConstructionScript`)